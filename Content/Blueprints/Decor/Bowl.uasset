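; Decor Blueprint for a food bowl that a cat can interact with to eat.
; InteractWithCat overrides the parent's function and, while the Food component is visible, stops the cat's movement and switches its sprite to the eating flipbook.
; EndofInteraction then waits briefly, hides the food and lets the cat move again.
; Nothing in this Blueprint restores the food afterwards.
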(event Custom|End%20of%20Interaction
  (params (Cat :type Paper%202D%20Cat%20Object%20Reference))
  ;[0.15 0.15 0.15 0.5] Deal with the end of the Interaction
  (Utilities|FlowControl|Delay 2.0)
  (CallFunction|ConsumeFood)
  ;;[0.15 0.15 0.15 0.5] The Cat can Move Again
  (Variables|/Game/Blueprints/Character/Paper2D_Cat.Paper2D_Cat_C|SetcanMove Cat true)
  (Development|PrintText "Ate"))

(event Custom|ConsumeFood
  ;[0.15 0.15 0.15 0.5] Make the bowl food disappear
  (Rendering|SetVisibility (Variables|Default|GetFood) false false))

(event EventBeginPlay
  (|CallParentFunction) ; Ce nœud est désactivé et ne sera pas appelé.\nFaites glisser les broches pour générer des fonctionnalités.
)

(event Collision|EventActorBeginOverlap
  (params (OtherActor :type Actor%20Object%20Reference))
  (|CallParentFunction OtherActor) ; Ce nœud est désactivé et ne sera pas appelé.\nFaites glisser les broches pour générer des fonctionnalités.
)

(event EventTick
  (params (DeltaSeconds :type Float%20%28single-precision%29))
  (|CallParentFunction DeltaSeconds) ; Ce nœud est désactivé et ne sera pas appelé.\nFaites glisser les broches pour générer des fonctionnalités.
)

(fn ConstructionScript
  (|CallParentFunction))

(fn InteractwithCat
  (params (cat :type Paper%202D%20Cat%20Object%20Reference))
  ;[0.15 0.15 0.15 0.5] Allow Cat to Eat Food
  (|CallParentFunction cat)
  (if (Rendering|IsVisible (Variables|Default|GetFood))
    (Variables|/Game/Blueprints/Character/Paper2D_Cat.Paper2D_Cat_C|SetcanMove cat false)
    (Sprite|SetFlipbook (Variables|/Script/Paper2D.PaperCharacter|GetSprite cat) "/Game/Models/Cat/Sprites/Eat/Anim_Cat_Eat.Anim_Cat_Eat")
    (CallFunction|EndOfInteraction cat)))