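; Food bowl decor actor that lets the player's cat eat when it is close enough.
; When a Paper2D_Cat overlaps it while the Food component is visible, it sets the cat's CanEat flag and passes itself as BowlRef.
; When the cat leaves the overlap, CanEat is cleared; both transitions print debug messages.
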(event EventBeginPlay)

(event EventTick
  (params (DeltaSeconds :type Float%20%28single-precision%29)))

(event Collision|EventActorBeginOverlap
  (params (OtherActor :type Actor%20Object%20Reference))
  ;[0.15 0.15 0.15 0.5] Allow Cat to Eat if Close enough
  (bind _aspaper_2d_cat (Utilities|Casting|CastToPaper2D_Cat OtherActor))
  (if (Rendering|IsVisible (Variables|Default|GetFood))
    (Variables|/Game/Blueprints/Character/Paper2D_Cat.Paper2D_Cat_C|SetcanEat _aspaper_2d_cat true)
    (Variables|/Game/Blueprints/Character/Paper2D_Cat.Paper2D_Cat_C|SetBowlRef _aspaper_2d_cat self)
    (Development|PrintString "Can Eat")))

(event Collision|EventActorEndOverlap
  (params (OtherActor :type Actor%20Object%20Reference))
  ;[0.15 0.15 0.15 0.5] Allow Cat to Eat if Close enough
  (bind _aspaper_2d_cat (Utilities|Casting|CastToPaper2D_Cat OtherActor))
  (Variables|/Game/Blueprints/Character/Paper2D_Cat.Paper2D_Cat_C|SetcanEat _aspaper_2d_cat false)
  (Development|PrintString "Can NOT Eat"))

(fn ConstructionScript)