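; InteractiveObject is a decor actor that the Paper2D_Cat character can interact with when close enough.
; Beginning overlap sets the cat's CanInteract flag and registers this object as its CloserInteractivObject, while ending overlap clears only the flag, each printing a debug message.
; InteractWithCat takes the cat but is empty here, and the event graph's "Basic Interaction" print is unreachable.
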(event EventBeginPlay)

(event EventTick
  (params (DeltaSeconds :type Float%20%28single-precision%29)))

(event Collision|EventActorBeginOverlap
  (params (OtherActor :type Actor%20Object%20Reference))
  ;[0.15 0.15 0.15 0.5] Allow Cat to Interact if Close enough
  (bind _aspaper_2d_cat (Utilities|Casting|CastToPaper2D_Cat OtherActor))
  (Variables|/Game/Blueprints/Character/Paper2D_Cat.Paper2D_Cat_C|SetcanInteract _aspaper_2d_cat true)
  (Variables|/Game/Blueprints/Character/Paper2D_Cat.Paper2D_Cat_C|SetCloserInteractivObject _aspaper_2d_cat self)
  (Development|PrintString "Can Interact"))

(event Collision|EventActorEndOverlap
  (params (OtherActor :type Actor%20Object%20Reference))
  ;[0.15 0.15 0.15 0.5] Allow Cat to Interact if Close enough
  (bind _aspaper_2d_cat (Utilities|Casting|CastToPaper2D_Cat OtherActor))
  (Variables|/Game/Blueprints/Character/Paper2D_Cat.Paper2D_Cat_C|SetcanInteract _aspaper_2d_cat false)
  (Development|PrintString "Can NOT Interact"))

(fn ConstructionScript)

(fn InteractwithCat
  (params (cat :type Paper%202D%20Cat%20Object%20Reference)))